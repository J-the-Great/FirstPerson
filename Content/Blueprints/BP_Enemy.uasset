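; BP_Enemy is an enemy that chases the player on sight and can be destroyed by a smote event.
; Pawn sensing sets a seen flag and starts an AI move to the player, with a montage play call on arrival that has no montage assigned.
; The seen flag is never cleared and the attack cooldown is never set true, so it gates nothing.
; Patrol is an empty stub.
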(event OnSeePawn(PawnSensing)
  (params (Pawn :type Pawn%20Object%20Reference))
  (Variables|Default|Setis%20seeing%20player true)
  (CallFunction|FollowPlayer))

(event Custom|FollowPlayer
  (Variables|Default|SetAttackCooldown false)
  (if (Variables|Default|Getis%20seeing%20player)
    (AI|AIMoveTo self "0, 0, 0" (Game|Player|GetPlayerPawn 0) 2e+01 false
      (:OnSuccess
        (if (not (Variables|Default|GetAttackCooldown))
          (Animation|PlayAnimMontage 0 1.0 "None"))))))

(event Custom|Patrol)

(event Custom|smote
  (Development|PrintString "smite")
  (Actor|DestroyActor))

(event EventBeginPlay)

(event Collision|EventActorBeginOverlap
  (params (OtherActor :type Actor%20Object%20Reference)))

(event EventTick
  (params (DeltaSeconds :type Float%20%28single-precision%29))
  (if true
    _))

(fn ConstructionScript)